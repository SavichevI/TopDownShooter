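; Top-down main character Blueprint with an adjustable boom camera and a key-triggered camera shake.
; The construction script applies exposed-style variables to the camera boom's lag, arm length and relative rotation.
; Pressing F plays a world camera shake centered on the top-down camera.
; Logic to yaw the character toward the cursor hit point exists but is disconnected, and Tick is empty.
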(event `Key|F`
  (params (Key :type "Key Structure"))
  (:`Pressed`
    (`GameplayStatics.PlayWorldCameraShake` "/Game/Blueprints/Game/BP_Camepa_Shake.BP_Camepa_Shake_C" (`SceneComponent.K2_GetComponentLocation` (`self.TopDownCameraComponent`)) 0.0 30.0)))

(event `self.ReceiveTick`
  (params (DeltaSeconds :type "Float (single-precision)")))

(fn `UserConstructionScript`
  (bind _cameraboom (`self.CameraBoom`))
  (set `SpringArmComponent.bEnableCameraLag` (`self.Flow`) _cameraboom)
  (set `SpringArmComponent.CameraLagSpeed` (`self.CameraLagSpeed`) _cameraboom)
  (set `SpringArmComponent.TargetArmLength` (`self.Hieght`) _cameraboom)
  (`SceneComponent.K2_SetRelativeRotation` _cameraboom (`self.RotatorCamera`) false false))